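; CarSpawner_BP is a spawner that creates TestCar actors, starting with one at the world origin on BeginPlay.
; SpawnCar stores the latest car in NewCar and hands that car a reference back to the spawner.
; SpawnCarAtSpawnPoint chains spawns by placing the next car at the world location of the latest car's SpawnPoint, though nothing in this Blueprint calls it.
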(event `self.ReceiveBeginPlay`
  (`self.SpawnCar` (0.0 0.0 0.0)))

(fn `SpawnCar`
  (params (SpawnLocation :type "Vector Structure"))
  (bind _returnvalue (`|SpawnActorFromClass` "/Game/Blueprints/TestCar.TestCar_C" (`KismetMathLibrary.MakeTransform` SpawnLocation) "Undefined" "OverrideRootScale" null null))
  (bind _output_get (set `self.NewCar` _returnvalue))
  (set `/Game/Blueprints/TestCar.CarSpawner` self _output_get))

(fn `SpawnCarAtSpawnPoint`
  (`self.SpawnCar` (`SceneComponent.K2_GetComponentLocation` (`/Game/Blueprints/TestCar.SpawnPoint` (`self.NewCar`)))))

(fn `UserConstructionScript`)