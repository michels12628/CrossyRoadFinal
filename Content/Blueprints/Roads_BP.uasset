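; Road segment Blueprint for a Crossy Road-style game that asks its RoadSpawner for another road when the player character enters its trigger zone.
; ChangeLanes stores the lane type and swaps the road mesh between grass, highway and tracks.
; SpawnBoundaries places obstacle actors with random tree meshes at the left and right boundary points, though nothing here calls it.
; Vehicle randomization and car spawning are unfinished, with their logic left unconnected.
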(event `self.TriggerZone.OnComponentBeginOverlap`
  (params (OverlappedComponent :type "PrimitiveComponent Object Reference") (OtherActor :type "Actor Object Reference") (OtherComp :type "PrimitiveComponent Object Reference") (OtherBodyIndex :type Integer) (bFromSweep :type Boolean) (SweepResult :type "HitResult Structure (by ref)"))
  (cast `/Game/Blueprints/Character_BP` OtherActor)
  (`/Game/Blueprints/SpawnRoads_BP.SpawnRoadatSpawnPoint` (`self.RoadSpawner`)))

(fn `ChangeLanes`
  (params (LaneType :type Integer))
  (bind _output_get (set `self.LaneType` LaneType))
  (`StaticMeshComponent.SetStaticMesh` (`self.Road`) (select `int` _output_get :`0` "/Game/Objects/crossyroad_grass.crossyroad_grass" :`1` "/Game/Objects/crossyroad_highway.crossyroad_highway" :`2` "/Game/Objects/crossyroad_tracks.crossyroad_tracks" :!type "StaticMesh Object Reference"))
  (switch `int` (`local.LaneType`)))

(fn `RandomizeVehicles`)

(fn `Spawn Cars`
  (params (Location :type "Vector Structure")))

(fn `SpawnBoundaries`
  (`self.SpawnObjects` (`SceneComponent.K2_GetComponentLocation` (`self.BoundaryLeft`)))
  (`self.SpawnObjects` (`SceneComponent.K2_GetComponentLocation` (`self.BoundaryRight`))))

(fn `SpawnObjects`
  (params (Location :type "Vector Structure"))
  (bind _returnvalue (`|SpawnActorFromClass` "/Game/Blueprints/Obstacle_BP.Obstacle_BP_C" (`KismetMathLibrary.Conv_VectorToTransform` Location) "Undefined" "OverrideRootScale" self null))
  (`StaticMeshComponent.SetStaticMesh` (`/Game/Blueprints/Obstacle_BP.StaticMesh` _returnvalue) (select `int` (`KismetMathLibrary.RandomIntegerInRange` 0 1) :`0` "/Game/Objects/crossyroad_pinetree.crossyroad_pinetree" :`1` "/Game/Objects/crossyroad_tree.crossyroad_tree" :!type "StaticMesh Object Reference")))

(fn `UserConstructionScript`)