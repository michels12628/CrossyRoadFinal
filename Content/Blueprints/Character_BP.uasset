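; Player chicken character that hops in four directions, crouching while W, A, S or D is held and launching along fixed world axes on release.
; Each hop increments JumpCount, and C toggles between the Camera and FPCamera views.
; Tick consumes movement input while alive; when DeadChicken is set, it disables movement and swaps in a flattened mesh.
; The NumberJumps counter function is left unused.
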(event `self.ReceiveBeginPlay`)

(event `Key|W`
  (params (Key :type "Key Structure"))
  (:`Pressed`
    (`self.Crouch`))
  (:`Released`
    (`self.UnCrouch`)
    (`self.LaunchCharacter` (250.0 0.0 300.0))
    (set `self.JumpCount` (+ (`self.JumpCount`) 1))))

(event `Key|S`
  (params (Key :type "Key Structure"))
  (:`Pressed`
    (`self.Crouch`))
  (:`Released`
    (`self.UnCrouch`)
    (`self.LaunchCharacter` (-250.0 0.0 300.0))
    (set `self.JumpCount` (+ (`self.JumpCount`) 1))))

(event `self.ReceiveTick`
  (params (DeltaSeconds :type "Float (single-precision)"))
  (if (`self.DeadChicken`)
    (`CharacterMovementComponent.DisableMovement` (`self.CharacterMovement`))
    (`StaticMeshComponent.SetStaticMesh` (`self.ChickenMesh`) "/Game/Objects/flatChicken.flatChicken")
    (else
      (`self.ConsumeMovementInputVector`))))

(event `Key|A`
  (params (Key :type "Key Structure"))
  (:`Pressed`
    (`self.Crouch`))
  (:`Released`
    (`self.UnCrouch`)
    (`self.LaunchCharacter` (0.0 -250.0 300.0))
    (set `self.JumpCount` (+ (`self.JumpCount`) 1))))

(event `InputAxis|MoveForwardBackward`
  (params (AxisValue :type "Float (single-precision)"))
  (bind (_returnvalue_roll _returnvalue_pitch) (`KismetMathLibrary.BreakRotator` (`self.K2_GetActorRotation`)))
  ;[1 1 1] Movement
  (`self.AddMovementInput` (`KismetMathLibrary.GetForwardVector` (`KismetMathLibrary.MakeRotator` _returnvalue_roll _returnvalue_pitch)) AxisValue))

(event `Key|D`
  (params (Key :type "Key Structure"))
  (:`Pressed`
    (`self.Crouch`))
  (:`Released`
    (`self.UnCrouch`)
    (`self.LaunchCharacter` (0.0 250.0 300.0))
    (set `self.JumpCount` (+ (`self.JumpCount`) 1))))

(event `InputAxis|MoveLeftRght`
  (params (AxisValue :type "Float (single-precision)"))
  (bind (_returnvalue_roll _returnvalue_pitch) (`KismetMathLibrary.BreakRotator` (`self.K2_GetActorRotation`)))
  ;[1 1 1] Movement
  (`self.AddMovementInput` (`KismetMathLibrary.GetRightVector` (`KismetMathLibrary.MakeRotator` _returnvalue_roll _returnvalue_pitch)) AxisValue))

(event `InputAction|Jump`
  (params (Key :type "Key Structure"))
  ;[1 1 1] Jump Test
)

(event `Key|C`
  (params (Key :type "Key Structure"))
  ;[1 1 1] Third/First Person
  (:`Pressed`
    (`/Engine/EditorBlueprintResources/StandardMacros.FlipFlop`
      (:`A`
        (`ActorComponent.SetActive` (`self.Camera`) true false)
        (`ActorComponent.SetActive` (`self.FPCamera`) false true))
      (:`B`
        (`ActorComponent.SetActive` (`self.Camera`) false true)
        (`ActorComponent.SetActive` (`self.FPCamera`) true false)))))

(fn `NumberJumps`
  (if (or (`self.WReleased`) (`self.AReleased`) (`self.SReleased`) (`self.DReleased`))
    (set `self.JumpCount` (+ (`self.JumpCount`) 1))
    (`KismetSystemLibrary.PrintString` (`KismetStringLibrary.Conv_IntToString` (`self.JumpCount`)))))

(fn `UserConstructionScript`)