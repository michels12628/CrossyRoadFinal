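; SpawnRoads_BP is a spawner actor that builds the chain of road segments when play begins.
; BeginPlay runs a fixed loop, placing the first Roads_BP at a set location and each next one at the newest road's SpawnPoint.
; Each road receives a reference to the spawner, a random ChangeLanes value and spawned boundaries.
; A RandomizeVehicles call is left unconnected and never runs.
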(event `self.ReceiveBeginPlay`
  (`self.SpawnInitialRoads`))

(fn `SpawnInitialRoads`
  (for _ (range 31)
    (`/Engine/EditorBlueprintResources/StandardMacros.IsValid` (`self.NewestRoad`)
      (:`Is Valid`
        (`self.SpawnRoadatSpawnPoint`))
      (:`Is Not Valid`
        (`self.SpawnRoad` (-925.0 0.0 0.0))))))

(fn `SpawnRoad`
  (params (SpawnLocation :type "Vector Structure"))
  (bind _returnvalue (`|SpawnActorFromClass` "/Game/Blueprints/Roads_BP.Roads_BP_C" (`KismetMathLibrary.MakeTransform` SpawnLocation) "Undefined" "OverrideRootScale" null null))
  (bind _output_get (set `self.NewestRoad` _returnvalue))
  ;[1 1 1] RefToSpawnRoads
  (set `/Game/Blueprints/Roads_BP.RoadSpawner` self _output_get)
  (`/Game/Blueprints/Roads_BP.ChangeLanes` _output_get (`KismetMathLibrary.RandomIntegerInRange` 0 1))
  (`/Game/Blueprints/Roads_BP.SpawnBoundaries` _output_get))

(fn `SpawnRoadatSpawnPoint`
  ;[1 1 1] SpawnNewTunnel
  (`self.SpawnRoad` (`SceneComponent.K2_GetComponentLocation` (`/Game/Blueprints/Roads_BP.SpawnPoint` (`self.NewestRoad`)))))

(fn `UserConstructionScript`)